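; Blood Curse spell actor that damages player characters (BP_ThirdPersonCharacter) overlapping its two collider zones.
; Entering InnerCollider applies full damage through MakeDamage and sets HasHitInner.
; Entering OuterCollider applies half damage unless that flag is set, then clears it.
; The single shared flag prevents double hits only when the inner overlap fires before the outer one.
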(event `self.InnerCollider.OnComponentBeginOverlap`
  (params (OverlappedComponent :type "PrimitiveComponent Object Reference") (OtherActor :type "Actor Object Reference") (OtherComp :type "PrimitiveComponent Object Reference") (OtherBodyIndex :type Integer) (bFromSweep :type Boolean) (SweepResult :type "HitResult Structure (by ref)"))
  (bind _asbp_third_person_character (cast `/Game/ThirdPerson/Blueprints/BP_ThirdPersonCharacter` OtherActor))
  (set `self.HasHitInner` true)
  (`self.MakeDamage` 1.0 _asbp_third_person_character))

(event `self.OuterCollider.OnComponentBeginOverlap`
  (params (OverlappedComponent :type "PrimitiveComponent Object Reference") (OtherActor :type "Actor Object Reference") (OtherComp :type "PrimitiveComponent Object Reference") (OtherBodyIndex :type Integer) (bFromSweep :type Boolean) (SweepResult :type "HitResult Structure (by ref)"))
  (bind _asbp_third_person_character (cast `/Game/ThirdPerson/Blueprints/BP_ThirdPersonCharacter` OtherActor))
  (if (not (`self.HasHitInner`))
    (`self.MakeDamage` 0.5 _asbp_third_person_character))
  (set `self.HasHitInner` false))

(fn `UserConstructionScript`
  (`parent.UserConstructionScript`))