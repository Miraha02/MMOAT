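; BP_Spell is a spell actor that gates itself on caster mana and provides damage logic through the Gameplay Ability System.
; On BeginPlay it destroys itself if a BP_MMOATCharacter caster lacks ManaCost; other casters always pass.
; MakeDamage applies GE_TakeDamage with negated Damage as a Skill.Damage set-by-caller magnitude, then calls the target's health and caster's mana change handlers.
; The GE_ManaCost spec is unconnected, so no mana is deducted here.
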(event `self.ReceiveBeginPlay`
  (bind _cancast (`self.hasEnoughMana`))
  (if (not _cancast)
    (`KismetSystemLibrary.PrintString` "Pas assez de mana (Message à implémenter)")
    (`self.K2_DestroyActor`)))

(event `DestroyActor`)

(event `self.ReceiveTick`
  (params (DeltaSeconds :type "Float (single-precision)")))

(event `self.ReceiveActorBeginOverlap`
  (params (OtherActor :type "Actor Object Reference")))

(fn `hasEnoughMana`
  (returns (CanCast :type Boolean))
  (bind _asbp_third_person_character (cast `/Game/ThirdPerson/Blueprints/BP_MMOATCharacter` (`self.Caster`))
    (:`then`
      (return (>= (`.ReturnValue` (`AbilitySystemComponent.GetGameplayAttributeValue` (`AbilitySystemBlueprintLibrary.GetAbilitySystemComponent` _asbp_third_person_character) (struct :`AttributeName` "Mana" :`Attribute` "/Script/MMOAT.CharacterAttributeSet:Mana" :`AttributeOwner` "/Script/CoreUObject.Class'/Script/MMOAT.CharacterAttributeSet'"))) (`self.ManaCost`))))
    (:`CastFailed`
      (return true))))

(fn `MakeDamage`
  (params (Caster :type "/Game/ThirdPerson/Blueprints/BP_MMOATCharacter Object Reference (by ref)") (Target :type "/Game/ThirdPerson/Blueprints/BP_MMOATCharacter Object Reference (by ref)"))
  (bind _returnvalue (`AbilitySystemBlueprintLibrary.GetAbilitySystemComponent` Caster))
  (`/Engine/EditorBlueprintResources/StandardMacros.IsValid` Caster
    (:`Is Valid`
      (bind _returnvalue_2 (`AbilitySystemBlueprintLibrary.AssignTagSetByCallerMagnitude` (`AbilitySystemComponent.MakeOutgoingSpec` :`self` _returnvalue :`GameplayEffectClass` "/Game/Blueprint/GAS/GE/GE_TakeDamage.GE_TakeDamage_C") (struct :`TagName` "Skill.Damage") (* (`self.Damage`) -1.0)))
      (`AbilitySystemComponent.BP_ApplyGameplayEffectSpecToTarget` _returnvalue _returnvalue_2 (`AbilitySystemBlueprintLibrary.GetAbilitySystemComponent` Target))
      (`/Game/ThirdPerson/Blueprints/BP_MMOATCharacter.OnHealthChanged` Target)
      (`/Game/ThirdPerson/Blueprints/BP_MMOATCharacter.OnManaChanged` Caster))))

(fn `UserConstructionScript`)