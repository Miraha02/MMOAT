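; BP_TargetedSpell is a targeted spell actor that lives briefly in the world and deals no damage itself in this graph.
; BeginPlay runs the parent logic, then starts a timer that destroys the actor after three seconds.
; Tick switches actor collision off every frame.
; The overlap event is empty, leaving the MakeDamage path on BP_MMOATCharacter disconnected; a TODO references other spells.
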(event `self.ReceiveBeginPlay`
  ;[1 1 1] TODO pour les autres spells
  (`parent.ReceiveBeginPlay`)
  (`KismetSystemLibrary.K2_SetTimerDelegate` (delegate `DestroyEvent`) 3.0))

(event `DestroyEvent`
  ;[1 1 1] TODO pour les autres spells
  (`self.K2_DestroyActor`))

(event `self.ReceiveTick`
  (params (DeltaSeconds :type "Float (single-precision)"))
  ;[1 1 1] TODO pour les autres spells
  (`parent.ReceiveTick` 0.0)
  (`self.SetActorEnableCollision` false))

(event `self.ReceiveActorBeginOverlap`
  (params (OtherActor :type "Actor Object Reference"))
  ;[1 1 1] TODO pour les autres spells
)

(fn `UserConstructionScript`
  (`parent.UserConstructionScript`))