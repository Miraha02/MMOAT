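; Gameplay ability that casts a spell by spawning the first class in the third-person character's SpellClasses0 array.
; On activation, it spawns the actor 500 units horizontally along a direction vector from the character, then immediately ends.
; The Lock flag selects that direction: forward plus up of the camera's first child component when set, otherwise the character's forward.
; The spawn transform carries location only, adjusted for collisions but always spawning.
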(event `self.K2_ActivateAbility`
  ;[1 1 1] CastUnSpell
  (bind _asbp_third_person_character (cast `/Game/ThirdPerson/Blueprints/BP_ThirdPersonCharacter` (`self.GetAvatarActorFromActorInfo`)))
  (bind _returnvalue (`SceneComponent.K2_GetComponentRotation` (`SceneComponent.GetChildComponent` (`/Game/ThirdPerson/Blueprints/BP_ThirdPersonCharacter.Camera` _asbp_third_person_character) 0)))
  (`|SpawnActorFromClass` (`|GetArrayItem` (`/Game/ThirdPerson/Blueprints/BP_ThirdPersonCharacter.SpellClasses_0` _asbp_third_person_character)) (`KismetMathLibrary.Conv_VectorToTransform` (+ (`Actor.K2_GetActorLocation` _asbp_third_person_character) (* (`KismetMathLibrary.SelectVector` (+ (`KismetMathLibrary.GetForwardVector` _returnvalue) (`KismetMathLibrary.GetUpVector` _returnvalue)) (`KismetMathLibrary.GetForwardVector` (`Actor.K2_GetActorRotation` _asbp_third_person_character)) (`/Game/ThirdPerson/Blueprints/BP_ThirdPersonCharacter.Lock` _asbp_third_person_character)) (500.0 500.0 1.0)))) "AdjustIfPossibleButAlwaysSpawn" "MultiplyWithRoot" null null)
  (`self.K2_EndAbility`))