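; Gameplay ability that casts the caster's selected spell on their locked target.
; Activation defers to the parent; CastSpell checks lock and short range, then spawns the indexed spell class at the target.
; The spawned spell calls its mana check, but the result does not gate MakeDamage, after which the ability ends.
; Without a lock it prints a placeholder message; that path and out-of-range casts never call EndAbility.
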(event `self.K2_ActivateAbility`
  (`parent.K2_ActivateAbility`))

(fn `CastSpell`
  (params (Caster :type "/Game/ThirdPerson/Blueprints/BP_MMOATCharacter Object Reference"))
  (bind _lockedactor (`/Game/ThirdPerson/Blueprints/BP_MMOATCharacter.LockedActor` Caster))
  (bind _returnvalue (`SceneComponent.K2_GetComponentLocation` (`Actor.RootComponent` _lockedactor)))
  ;[1 1 1] Check si un actor est locked
  (if (`KismetSystemLibrary.IsValid` (`/Game/ThirdPerson/Blueprints/BP_MMOATCharacter.LockedActor` Caster))
    ;[1 1 1] Check si l'ennemy est dans la range
    (if (< (`KismetMathLibrary.Vector_Distance` (`SceneComponent.K2_GetComponentLocation` (`Character.Mesh` Caster)) _returnvalue) 500.0)
      (bind _returnvalue_2 (`|SpawnActorFromClass` (`|GetArrayItem` (`/Game/ThirdPerson/Blueprints/BP_MMOATCharacter.SpellClasses` Caster) (`/Game/ThirdPerson/Blueprints/BP_MMOATCharacter.SpellIndex` Caster)) (`KismetMathLibrary.Conv_VectorToTransform` _returnvalue) "AdjustIfPossibleButAlwaysSpawn" "MultiplyWithRoot" null null))
      (bind _output_get (set `/Game/Blueprint/Spells/BP_Spell.Caster` Caster _returnvalue_2))
      (`/Engine/EditorBlueprintResources/StandardMacros.IsValid` _output_get
        (:`Is Valid`
          (`/Game/Blueprint/Spells/BP_Spell.hasEnoughMana` _returnvalue_2)
          (if true
            (`/Game/Blueprint/Spells/BP_Spell.MakeDamage` _returnvalue_2 _output_get _lockedactor)
            (`self.K2_EndAbility`)))))
    (else
      (`KismetSystemLibrary.PrintString` "T'as pas lock de target bouffon (message à implémenter)"))))