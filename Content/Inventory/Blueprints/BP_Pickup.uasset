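; World pickup actor for an inventory item, showing its mesh and name and letting a player collect it.
; An ID rep-notify, also run at construction and BeginPlay, loads the DT_Inventory row or uses DropItem if set, then blocking-loads a skeletal mesh, falling back to static.
; Sphere overlap by the local non-AI player toggles the name widget and registers it with MMOPlayerController.
; Interact sets the owner and forwards pickup to the controlled pawn.
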(event `Destroy`
  (`self.K2_DestroyActor`))

(event `self.ReceiveBeginPlay`
  (`self.OnRep_ID`))

(event `Update`
  (bind ((`DisplayName_9_F6ABBA35434AB10F914060BF57038C4A` _displayname) (`PickupMesh_25_64A7E3E64AFCDE3ACFC5D3BFD52AC3F1` _pickupmesh) (`PickupMeshStatic_28_5186EA314C989E83D7B6F79F1CB07C51` _pickupmeshstatic)) (break `/Game/Inventory/Data/ST_Inventory_Item` (`self.Item`)))
  (bind _aswb_pickup (cast `/Game/Inventory/Widgets/WB_Pickup` (`WidgetComponent.GetWidget` (`self.Widget`))))
  (`TextBlock.SetText` (`/Game/Inventory/Widgets/WB_Pickup.Text` _aswb_pickup) _displayname)
  (bind _returnvalue (`KismetSystemLibrary.LoadAsset_Blocking` _pickupmesh))
  (bind _asskeletal_mesh (cast `SkeletalMesh` _returnvalue)
    (:`then`
      (`SkinnedMeshComponent.SetSkinnedAssetAndUpdate` (`self.SkeletalMesh`) _asskeletal_mesh true))
    (:`CastFailed`
      (bind _returnvalue_2 (`KismetSystemLibrary.LoadAsset_Blocking` _pickupmeshstatic))
      (bind _asstatic_mesh (cast `StaticMesh` _returnvalue_2))
      (`StaticMeshComponent.SetStaticMesh` (`self.StaticMesh`) _asstatic_mesh))))

(event `self.Sphere.OnComponentBeginOverlap`
  (params (OverlappedComponent :type "PrimitiveComponent Object Reference") (OtherActor :type "Actor Object Reference") (OtherComp :type "PrimitiveComponent Object Reference") (OtherBodyIndex :type Integer) (bFromSweep :type Boolean) (SweepResult :type "HitResult Structure (by ref)"))
  (bind _ascharacter (cast `Character` OtherActor))
  (`self.IsPlayer` _ascharacter
    (:`true`
      (`SceneComponent.SetVisibility` (`self.Widget`) true false)
      (bind _asmmoplayer_controller (cast `MMOPlayerController` (`Pawn.GetController` _ascharacter)))
      (`MMOPlayerController.AddInteractable` _asmmoplayer_controller self))))

(event `self.Sphere.OnComponentEndOverlap`
  (params (OverlappedComponent :type "PrimitiveComponent Object Reference") (OtherActor :type "Actor Object Reference") (OtherComp :type "PrimitiveComponent Object Reference") (OtherBodyIndex :type Integer))
  (bind _ascharacter (cast `Character` OtherActor))
  (`self.IsPlayer` _ascharacter
    (:`true`
      (`SceneComponent.SetVisibility` (`self.Widget`) false false)
      (bind _asmmoplayer_controller (cast `MMOPlayerController` (`Pawn.GetController` _ascharacter)))
      (`MMOPlayerController.RemoveInteractable` _asmmoplayer_controller self))))

(fn `Interact`
  (params (Interactor :type "Actor Object Reference"))
  (returns (ReturnValue :type Boolean))
  (bind _ascontroller (cast `Controller` Interactor))
  (`self.SetOwner` _ascontroller)
  (bind _success (message `/Game/Inventory/Blueprints/BPI_Inventory.PickupItem` (`Controller.K2_GetPawn` _ascontroller) (`self.ID`) (`self.DropItem`) self))
  (return _success))

(fn `OnRep_ID`
  (bind _returnvalue (`|GetDataTableRow` "/Game/Inventory/DT_Inventory.DT_Inventory" (`self.ID`))
    (:`then`
      (set `self.Item` (select `bool` (!= (`.ID_2_BAD5004A42257F6316AE9B8B68F02CF4` (break `/Game/Inventory/Data/ST_Inventory_Item` (`self.DropItem`))) "None") :`false` _returnvalue :`true` (`self.DropItem`)))
      (`self.Update`))))

(fn `UserConstructionScript`
  (`self.OnRep_ID`))